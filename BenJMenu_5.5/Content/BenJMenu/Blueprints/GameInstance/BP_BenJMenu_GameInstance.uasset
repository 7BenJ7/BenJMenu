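; Game instance for the BenJ menu that loads or creates the settings save at startup and applies it to colorblind mode, language and music/SFX volume.
; On first run it saves defaults and sets fullscreen, high scalability levels and a 60 FPS cap.
; It tracks gamepad use through input device connection changes and fires connect/disconnect dispatchers.
; A helper destroys EIK sessions and reopens the main menu with an error option.
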(event `InitializeSettingsData`
  (params (Target :type "/BenJMenu/BenJMenu/Blueprints/Save/BP_BenJMenu_SaveSettings Object Reference"))
  (bind _colorblindseverity (`/BenJMenu/BenJMenu/Blueprints/Save/BP_BenJMenu_SaveSettings.ColorblindSeverity` Target))
  (switch `int` (`/BenJMenu/BenJMenu/Blueprints/Save/BP_BenJMenu_SaveSettings.ColorblindIndex` Target)
    (:`0`
      (`WidgetBlueprintLibrary.SetColorVisionDeficiencyType` "NormalVision" _colorblindseverity))
    (:`1`
      (`WidgetBlueprintLibrary.SetColorVisionDeficiencyType` "Deuteranope" _colorblindseverity))
    (:`2`
      (`WidgetBlueprintLibrary.SetColorVisionDeficiencyType` "Protanope" _colorblindseverity))
    (:`3`
      (`WidgetBlueprintLibrary.SetColorVisionDeficiencyType` "Tritanope" _colorblindseverity)))
  (switch `int` (`/BenJMenu/BenJMenu/Blueprints/Save/BP_BenJMenu_SaveSettings.LanguageIndex` Target)
    (:`0`
      (`KismetInternationalizationLibrary.SetCurrentCulture` "en" true))
    (:`1`
      (`KismetInternationalizationLibrary.SetCurrentCulture` "fr-FR" true)))
  (`GameplayStatics.SetSoundMixClassOverride` "/BenJMenu/BenJMenu/Musics/SCM_Master.SCM_Master" "/BenJMenu/BenJMenu/Musics/SC_Music.SC_Music" (`/BenJMenu/BenJMenu/Blueprints/Save/BP_BenJMenu_SaveSettings.MusicVolume` Target) 1.0 0.0)
  (`GameplayStatics.PushSoundMixModifier` "/BenJMenu/BenJMenu/Musics/SCM_Master.SCM_Master")
  (`GameplayStatics.SetSoundMixClassOverride` "/BenJMenu/BenJMenu/Musics/SCM_Master.SCM_Master" "/BenJMenu/BenJMenu/Musics/SC_VFX.SC_VFX" (`/BenJMenu/BenJMenu/Blueprints/Save/BP_BenJMenu_SaveSettings.SFXVolume` Target) 1.0 0.0)
  (`GameplayStatics.PushSoundMixModifier` "/BenJMenu/BenJMenu/Musics/SCM_Master.SCM_Master"))

(event `self.ReceiveInit`
  (add `self.OnInputDeviceConnectionChange` (delegate `UpdateDeviceConnection`))
  (bind _returnvalue (`GameplayStatics.DoesSaveGameExist` (`self.SettingsSaveSlotName`)))
  (if _returnvalue
    (bind _returnvalue_2 (`GameplayStatics.LoadGameFromSlot` (`self.SettingsSaveSlotName`)))
    (bind _asbp_ben_jmenu_save_settings (cast `/BenJMenu/BenJMenu/Blueprints/Save/BP_BenJMenu_SaveSettings` _returnvalue_2))
    (`self.InitializeSettingsData` _asbp_ben_jmenu_save_settings)
    (else
      (bind _returnvalue_3 (`GameplayStatics.CreateSaveGameObject` "/BenJMenu/BenJMenu/Blueprints/Save/BP_BenJMenu_SaveSettings.BP_BenJMenu_SaveSettings_C"))
      (set `/BenJMenu/BenJMenu/Blueprints/Save/BP_BenJMenu_SaveSettings.UseContrastMode` false _returnvalue_3)
      (set `/BenJMenu/BenJMenu/Blueprints/Save/BP_BenJMenu_SaveSettings.UseCameraShake` true _returnvalue_3)
      (set `/BenJMenu/BenJMenu/Blueprints/Save/BP_BenJMenu_SaveSettings.UseForceFeedback` true _returnvalue_3)
      (set `/BenJMenu/BenJMenu/Blueprints/Save/BP_BenJMenu_SaveSettings.MusicVolume` 1.0 _returnvalue_3)
      (set `/BenJMenu/BenJMenu/Blueprints/Save/BP_BenJMenu_SaveSettings.SFXVolume` 1.0 _returnvalue_3)
      (set `/BenJMenu/BenJMenu/Blueprints/Save/BP_BenJMenu_SaveSettings.ColorblindSeverity` 0.5 _returnvalue_3)
      (set `/BenJMenu/BenJMenu/Blueprints/Save/BP_BenJMenu_SaveSettings.GamepadIndex` 0 _returnvalue_3)
      (`GameplayStatics.SaveGameToSlot` _returnvalue_3 (`self.SettingsSaveSlotName`))
      (`self.InitializeSettingsData` _returnvalue_3)
      (bind _returnvalue_4 (`GameUserSettings.GetGameUserSettings`))
      (`GameUserSettings.SetFullscreenMode` _returnvalue_4 "Fullscreen")
      (`GameUserSettings.ApplySettings` _returnvalue_4 true)
      (bind _returnvalue_5 (`GameUserSettings.GetGameUserSettings`))
      (`|ExecutionSequence`
        (:`then_0`
          (`GameUserSettings.SetAntiAliasingQuality` _returnvalue_5 3))
        (:`then_1`
          (`GameUserSettings.SetAudioQualityLevel` _returnvalue_5 3))
        (:`then_2`
          (`GameUserSettings.SetGlobalIlluminationQuality` _returnvalue_5 3))
        (:`then_3`
          (`GameUserSettings.SetPostProcessingQuality` _returnvalue_5 3))
        (:`then_4`
          (`GameUserSettings.SetReflectionQuality` _returnvalue_5 3))
        (:`then_5`
          (`GameUserSettings.SetShadingQuality` _returnvalue_5 3))
        (:`then_6`
          (`GameUserSettings.SetShadowQuality` _returnvalue_5 3))
        (:`then_7`
          (`GameUserSettings.SetTextureQuality` _returnvalue_5 3))
        (:`then_8`
          (`GameUserSettings.SetFrameRateLimit` _returnvalue_5 60.0)))
      (`GameUserSettings.ApplySettings` _returnvalue_5 true))))

(event `UpdateDeviceConnection` :!signature `self.OnInputDeviceConnectionChange`
  (params (NewConnectionState :type "EInputDeviceConnectionState Enum" :default "Invalid") (PlatformUserId :type "PlatformUserId Structure") (InputDeviceId :type "InputDeviceId Structure"))
  (`KismetSystemLibrary.PrintString` (`KismetStringLibrary.Concat_StrStr` (`KismetStringLibrary.Conv_InputDeviceIdToString` InputDeviceId) "  //  " (`|GetEnumeratorNameAsString` NewConnectionState)))
  (switch `EInputDeviceConnectionState` NewConnectionState
    (:`Invalid`
      (set `self.IsUsingGamepad` false :!label _label)
      (`self.OnDeviceDisconnect`))
    (:`Unknown`
      (goto _label))
    (:`Disconnected`
      (goto _label))
    (:`Connected`
      (set `self.IsUsingGamepad` true)
      (`self.OnDeviceConnect`))))